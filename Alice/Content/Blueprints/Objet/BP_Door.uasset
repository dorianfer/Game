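; BP_Door is a keyed door that swings open or closed when a player enters its trigger box.
; On overlap, it checks whether the BP_Player has a key for the door's KeyChannel and, if so, toggles the Open state.
; A timeline drives the Door component's relative yaw, playing forward to open and reversing to close.
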(event OnComponentBeginOverlap(Box)
  (params (OverlappedComponent :type Primitive%20Component%20Object%20Reference) (OtherActor :type Actor%20Object%20Reference) (OtherComp :type Primitive%20Component%20Object%20Reference) (OtherBodyIndex :type Integer) (bFromSweep :type Boolean) (SweepResult :type Hit%20Result%20Structure%20%28by%20ref%29))
  (bind _asbp_player (Utilities|Casting|CastToBP_Player OtherActor))
  (Utilities|IsValid _asbp_player
    (:Is%20Valid
      (if (Default|HasKey? _asbp_player (Variables|Constants|GetKeyChannel))
        (if (Variables|Private|GetOpen?)
          (CallFunction|Close)
          (else
            (CallFunction|Open)))))))

(event Custom|Open
  (Variables|Private|SetOpen? true)
  (bind _door_rotation (Timeline|RotateDoor%20Timeline Play)
    (:Update
      (Transformation|SetRelativeRotation (Variables|Default|GetDoor) (Math|Rotator|MakeRotator 0.0 0.0 _door_rotation) false false))))

(event Custom|Close
  (Variables|Private|SetOpen? false)
  (bind _door_rotation (Timeline|RotateDoor%20Timeline Reverse)
    (:Update
      (Transformation|SetRelativeRotation (Variables|Default|GetDoor) (Math|Rotator|MakeRotator 0.0 0.0 _door_rotation) false false))))

(event EventBeginPlay)

(event Collision|EventActorBeginOverlap
  (params (OtherActor :type Actor%20Object%20Reference)))

(event EventTick
  (params (DeltaSeconds :type Float%20%28single-precision%29)))

(fn ConstructionScript)